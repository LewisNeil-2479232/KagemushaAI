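; Base enemy character that works with AIC_EnemyBase and its blackboard for patrol, senses, alertness and combat ranges.
; BPCDamageSystem handles health, with bone-group hit routing and conditional headshot kills; damage responses spawn blood and turn unaware enemies toward hits.
; Unarmed attacks play random punch montages with notify-driven, timer-looped hand sphere traces.
; Also handles look-around montages, sight light, weapon drop and pickup, and ragdoll death.
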(event `StopRotating`
  (bind _damagemovementdistance (`self.DamageMovementDistance`))
  ;[1 0 1] Damage
  (`KismetSystemLibrary.K2_ClearAndInvalidateTimerHandle` (`self.DamageRotationTimerHandle`))
  (bind _asaic_enemy_base (cast `/Game/Ai/AIC_EnemyBase` (`self.GetController`)))
  (`/Game/Ai/AIC_EnemyBase.HandleHearing` _asaic_enemy_base (`NavigationSystemV1.K2_ProjectPointToNavigation` (+ (`self.K2_GetActorLocation`) (* (`KismetMathLibrary.Vector_NormalUnsafe` (`KismetMathLibrary.MakeVector` (.x (stale `DamageResponse` DamageNormal)) (.y (stale `DamageResponse` DamageNormal)))) _damagemovementdistance)) null null (`KismetMathLibrary.Conv_DoubleToVector` _damagemovementdistance))))

(event `DamageResponse`
  (params (DamageResponse :type "/Game/Ai/DamageSystem/E_DamageResponse Enum" :default "NewEnumerator0") (DamageLocation :type "Vector Structure") (DamageNormal :type "Vector Structure"))
  ;[1 0 1] Damage
  (`/Game/Ai/BaseEnemy/BloodVFX/AC_Blood_Effect.BloodEffect` (`self.AC_Blood_Effect`) DamageLocation DamageNormal)
  (switch `/Game/Ai/DamageSystem/E_DamageResponse` DamageResponse
    (:`NewEnumerator0`
      _)
    (:`NewEnumerator1`
      _)
    (:`NewEnumerator2`
      _)
    (:`NewEnumerator3`
      _)
    (:`NewEnumerator4`
      _))
  (bind _asaic_enemy_base (cast `/Game/Ai/AIC_EnemyBase` (`self.GetController`)))
  (`/Game/Ai/AIC_EnemyBase.SetAlertnessSearching` _asaic_enemy_base)
  (bind _state (`/Game/Ai/AIC_EnemyBase.GetCurrentState` _asaic_enemy_base))
  (switch `/Game/Ai/BaseEnemy/EnemyBaseEnums/E_AiStates` _state
    (:`NewEnumerator0`
      _)
    (:`NewEnumerator2`
      _))
  (bind _returnvalue (`KismetSystemLibrary.K2_SetTimerDelegate` (delegate `RotateToFaceDamage`) 0.1 true))
  (set `self.DamageRotationTimerHandle` _returnvalue))

(event `self.ReceiveBeginPlay`
  ;[1 0 1] Begin Play
  (bind _asaic_enemy_base (cast `/Game/Ai/AIC_EnemyBase` (`self.GetController`)))
  (bind _blackboard (`AIController.Blackboard` _asaic_enemy_base))
  (`BlackboardComponent.SetValueAsBool` _blackboard (`self.Should Patrol Key Name`) (`self.bShouldPatrol`))
  (`BlackboardComponent.SetValueAsVector` _blackboard (`self.BeginningLocationKeyName`) (`self.K2_GetActorLocation`))
  (`BlackboardComponent.SetValueAsRotator` _blackboard (`self.BegginingRotationKeyName`) (`self.K2_GetActorRotation`))
  (`SceneComponent.K2_DetachFromComponent` (`self.PatrolPath`) "KeepWorld" "KeepWorld" "KeepWorld" true))

(event `RotateToFaceDamage`
  (bind (_returnvalue_roll _returnvalue_pitch _returnvalue_yaw) (`KismetMathLibrary.BreakRotator` (`self.K2_GetActorRotation`)))
  ;[1 0 1] Damage
  (bind (_returnvalue_roll_2 _returnvalue_pitch_2 _returnvalue_yaw_2) (`KismetMathLibrary.BreakRotator` (`KismetMathLibrary.Conv_VectorToRotator` (stale `DamageResponse` DamageNormal))))
  (bind _returnvalue (`KismetMathLibrary.MakeRotator` _returnvalue_roll_2 0.0 _returnvalue_yaw_2))
  (bind _returnvalue_2 (`KismetMathLibrary.RLerp` (`KismetMathLibrary.MakeRotator` _returnvalue_roll 0.0 _returnvalue_yaw) _returnvalue (`self.DamageRotationSpeed`) true))
  (`self.K2_SetActorRotation` _returnvalue_2)
  (if (== _returnvalue_2 _returnvalue :`ErrorTolerance` 20.0)
    (`self.StopRotating`)))

(event `Death`
  ;[1 0 1] Ragdoll + delete certain components + Drop weapon
  (`PrimitiveComponent.SetSimulatePhysics` (`self.Mesh`) true)
  (`PrimitiveComponent.SetCollisionEnabled` (`self.Mesh`) "QueryAndPhysics")
  (`PrimitiveComponent.SetCollisionEnabled` (`self.CapsuleComponent`) "NoCollision")
  (`self.TurnOffSightLight`)
  (bind _asaic_enemy_base (cast `/Game/Ai/AIC_EnemyBase` (`self.GetController`)))
  (`/Game/Ai/AIC_EnemyBase.AIDead` _asaic_enemy_base)
  (`KismetArrayLibrary.Array_Clear` (`self.Tags`))
  (`KismetArrayLibrary.Array_Add` (`self.Tags`) (`self.Tag Key Name`))
  (`self.Drop Weapon`))

(event `Drop Weapon`
  (bind _weaponactor (`self.WeaponActor`))
  (bind _weaponmesh (`/Game/Ai/Weapons/BP_AIWeapon_Base.WeaponMesh` _weaponactor))
  ;[1 0 1] Drop the weapon
  (`|ExecutionSequence`
    (:`then_0`
      (`self.K2_DetachFromActor` _weaponactor "KeepWorld" "KeepWorld" "KeepWorld")
      (`PrimitiveComponent.SetSimulatePhysics` _weaponmesh true)
      (`PrimitiveComponent.SetCollisionEnabled` _weaponmesh "QueryAndPhysics")
      (set `self.bIsWieldingWeapon` false)
      (set `self.bHasLostWeapon` true)
      (bind _asaic_enemy_base (cast `/Game/Ai/AIC_EnemyBase` (`self.GetController`)))
      (`BlackboardComponent.SetValueAsBool` (`AIController.Blackboard` _asaic_enemy_base) (`self.Has Weapon Key Name`) false)
      (set `self.Attack Radius` (`self.Mellee Attack Radius`))
      (set `self.Defend Radius` (`self.Mellee Defend Radius`))
      (bind _asaic_enemy_base_2 (cast `/Game/Ai/AIC_EnemyBase` (`self.GetController`)))
      (`/Game/Ai/AIC_EnemyBase.UpdateCombatRanges` _asaic_enemy_base_2))
    (:`then_1`
      (bind _asaic_enemy_base_3 (cast `/Game/Ai/AIC_EnemyBase` (`self.GetController`)))
      (bind _state (`/Game/Ai/AIC_EnemyBase.GetCurrentState` _asaic_enemy_base_3))
      (switch `/Game/Ai/BaseEnemy/EnemyBaseEnums/E_AiStates` _state
        (:`NewEnumerator0`
          _)
        (:`NewEnumerator2`
          _))
      (`|PlayMontage` (`self.Mesh`) "/Game/AnimRetarget/RT_DropWeapon.RT_DropWeapon"
        (:`then`
          (`self.TurnOffSightLight`))
        (:`OnCompleted`
          (`self.TurnOnSightLight`))))))

(event `Look Around`
  (params (Alertness :type "/Game/Ai/BaseEnemy/EnemyBaseEnums/E_AiAlertness Enum" :default "NewEnumerator0") (OwnerController :type "AIController Object Reference"))
  ;[1 0 1] Looking around
  (`KismetSystemLibrary.K2_SetTimer` OwnerController "MoveAIPerception" 0.1 true)
  (switch `/Game/Ai/BaseEnemy/EnemyBaseEnums/E_AiAlertness` Alertness
    (:`NewEnumerator0`
      (`|PlayMontage` (`self.Mesh`) "/Game/AnimRetarget/RT_Look_Around_Montage.RT_Look_Around_Montage"
        (:`OnCompleted`
          _)
        (:`OnInterrupted`
          _)))
    (:`NewEnumerator1`
      (`|PlayMontage` (`self.Mesh`) "/Game/AnimRetarget/RT_Nervously_Look_Around_Montage.RT_Nervously_Look_Around_Montage"
        (:`OnCompleted`
          _)
        (:`OnInterrupted`
          _)))
    (:`NewEnumerator2`
      _)
    (:`NewEnumerator3`
      _))
  (`self.OnLookAroundEnd`)
  (bind _asaic_enemy_base (cast `/Game/Ai/AIC_EnemyBase` (`self.GetController`)))
  (`BlackboardComponent.SetValueAsBool` (`AIController.Blackboard` _asaic_enemy_base) (`self.Should Look Around Key Name`) false))

(event `Pick Up Weapon`
  (bind (_projectedlocation _returnvalue) (`NavigationSystemV1.K2_ProjectPointToNavigation` (`SceneComponent.K2_GetComponentLocation` (`/Game/Ai/Weapons/BP_AIWeapon_Base.WeaponMesh` (`self.WeaponActor`)))))
  (if (`self.bHasLostWeapon`)
    (if _returnvalue
      (`|AIMoveTo` self _projectedlocation (`self.WeaponActor`) 50.0
        (:`OnSuccess`
          (set `self.bIsWieldingWeapon` true)
          (set `self.bHasLostWeapon` false)
          (`BlackboardComponent.SetValueAsBool` (`AIBlueprintHelperLibrary.GetBlackboard` (`self.GetController`)) (`self.Has Weapon Key Name`) true)
          (`self.K2_DestroyActor` (`self.WeaponActor`))
          (`self.EquipWeapon`)
          (bind _asaic_enemy_base (cast `/Game/Ai/AIC_EnemyBase` (`self.GetController`)))
          (`/Game/Ai/AIC_EnemyBase.UpdateCombatRanges` _asaic_enemy_base)))
      (else
        (set `self.bIsWieldingWeapon` false)
        (set `self.bHasLostWeapon` true)))))

(event `self.InstaAggroSight.OnSeePawn`
  (params (Pawn :type "Pawn Object Reference"))
  ;[1 0 1] Instantly see the player if they are too close
  (for _array_element (`Actor.Tags` Pawn)
    (switch `name` _array_element
      (:`Player`
        (bind _asaic_enemy_base (cast `/Game/Ai/AIC_EnemyBase` (`self.GetController`)))
        (set `/Game/Ai/AIC_EnemyBase.TimeSeenPlayer` (`/Game/Ai/AIC_EnemyBase.PerceptionMax` _asaic_enemy_base) _asaic_enemy_base)))))

(event `RotateSightBar`
  ;[1 0 1] Rotates the sight bar so its facing the player
  (`SceneComponent.K2_SetWorldRotation` (`self.SightBar`) (`KismetMathLibrary.MakeRotator` 0.0 0.0 -90.0) false false))

(event `AddAggressiveOverlay`
  ;[1 0 1] Overlay / Glow Effects
  (`MeshComponent.SetOverlayMaterial` (`self.Mesh`) "/Game/Ai/BaseEnemy/Materials/M_AggressiveAura.M_AggressiveAura")
  (`self.StopRotating`))

(event `RemoveGlows`
  ;[1 0 1] Overlay / Glow Effects
  (`MeshComponent.SetOverlayMaterial` (`self.Mesh`) null))

(event `TurnOnSightLight`
  ;[1 0 1] Spot Light effects
  (bind _asaic_enemy_base (cast `/Game/Ai/AIC_EnemyBase` (`self.GetController`)))
  (bind _state (`/Game/Ai/AIC_EnemyBase.GetCurrentState` _asaic_enemy_base))
  (switch `/Game/Ai/BaseEnemy/EnemyBaseEnums/E_AiStates` _state
    (:`NewEnumerator0`
      _)
    (:`NewEnumerator2`
      _))
  (`SceneComponent.SetVisibility` (`self.SightLight`) true true))

(event `TurnOffSightLight`
  ;[1 0 1] Spot Light effects
  (`SceneComponent.SetVisibility` (`self.SightLight`) false true))

(event `/Game/Ai/BPI_EnemyAi.Attack`
  ;[1 0 1] Attack + Hit Trace
  (if (not (`self.bIsWieldingWeapon`))
    (set `self.bUseControllerRotationYaw` false)
    ;;[0 1 1] Random Attack Selector
    (bind _newparam (`self.SelectMelee`))
    (bind _selectedattack (`self.RandomAttack` _newparam))
    (bind _notifyname (`|PlayMontage` (`self.Mesh`) _selectedattack)
      (:`OnCompleted`
        (set `self.bUseControllerRotationYaw` true :!label _label)
        (`self.OnAttackEnd`))
      (:`OnInterrupted`
        (goto _label))
      (:`OnNotifyBegin`
        (switch `name` _notifyname
          (:`StartTrace`
            (`self.StartFistTrace`))
          (:`StopTrace`
            (`KismetSystemLibrary.K2_ClearAndInvalidateTimerHandle` (`self.FistTraceTimerHandle`))))))))

(event `StartFistTrace`
  ;[1 0 1] Attack + Hit Trace
  (bind _returnvalue (`KismetSystemLibrary.K2_SetTimerDelegate` (delegate `FistTraceLoop`) 0.01 true))
  (set `self.FistTraceTimerHandle` _returnvalue))

(event `FistTraceLoop`
  (bind _returnvalue (`SceneComponent.K2_GetComponentLocation` (`self.HandSceneComponent`)))
  ;[1 0 1] Attack + Hit Trace
  (bind _outhits (`KismetSystemLibrary.SphereTraceMultiForObjects` :`Start` _returnvalue :`End` _returnvalue :`Radius` 20.0 :`ObjectTypes` (`|MakeArray` "ObjectTypeQuery3" :!type "EObjectTypeQuery Enum") :`DrawDebugType` "ForDuration"))
  (for _array_element _outhits
    (cast `SkeletalMeshComponent` (`.HitComponent` (`GameplayStatics.BreakHitResult` _array_element)))
    (bind (_bblockinghit _binitialoverlap _time _distance _location _impactpoint _normal _impactnormal _physmat _hitactor _hitcomponent _hitbonename) (`GameplayStatics.BreakHitResult` _array_element))
    (message `/Game/Ai/DamageSystem/BPI_Damageable.TakeDamage` _hitactor (make `/Game/Ai/DamageSystem/S_DamageInfo` 10.0 "NewEnumerator2" "NewEnumerator0" _impactpoint _impactnormal _hitbonename))
    (`KismetSystemLibrary.K2_ClearAndInvalidateTimerHandle` (`self.FistTraceTimerHandle`))
    (break)))

(fn `GetBoneGroup`
  (params (BoneHit :type Name))
  (returns (AreaHit :type Name))
  (bind _output_get (set `self.BoneHit` BoneHit))
  (if (`KismetArrayLibrary.Array_Contains` (`self.HeadBones`) _output_get)
    (return "Head")
    (elif (`KismetArrayLibrary.Array_Contains` (`self.LeftArmBones`) (`self.BoneHit`))
      (return "LeftArm")
      (elif (`KismetArrayLibrary.Array_Contains` (`self.RightArmBones`) (`self.BoneHit`))
        (return "RightArm")
        (elif (`KismetArrayLibrary.Array_Contains` (`self.LeftLegBones`) (`self.BoneHit`))
          (return "LeftLeg")
          (elif (`KismetArrayLibrary.Array_Contains` (`self.RightLegBones`) (`self.BoneHit`))
            (return "RightLeg")
            (elif (`KismetArrayLibrary.Array_Contains` (`self.StomachBones`) (`self.BoneHit`))
              (return "Stomach")
              (else
                (return "Other")))))))))

(fn `GetCurrentHealth`
  (returns (Health :type "Float (double-precision)"))
  (return (`/Game/Ai/DamageSystem/BPC_DamageSystem.Health` (`self.BPC_DamageSystem`))))

(fn `GetIdealRange`
  (returns (AttackRadius :type "Float (double-precision)") (DefendRadius :type "Float (double-precision)"))
  (return (`self.Attack Radius`) (`self.Defend Radius`)))

(fn `GetPatrolRoute`
  (returns (PatrolRoute :type "SplineComponent Object Reference"))
  (return (`self.PatrolPath`)))

(fn `RandomAttack`
  (params (AttackList :type "Array of AnimMontage Object Reference"))
  (returns (SelectedAttack :type "AnimMontage Object Reference"))
  (bind _output_get (set `self.SelectedAttack` (`|GetArrayItem` AttackList (`KismetMathLibrary.RandomIntegerInRange` 0 (- (`KismetArrayLibrary.Array_Length` AttackList) 1)))))
  (return _output_get))

(fn `SelectMelee`
  (returns (NewParam :type "Array of AnimMontage Object Reference"))
  (bind _luppercutpunch (`self.LUppercutPunch`))
  (if (`KismetMathLibrary.RandomBool`)
    (set `self.HandSceneComponent` (`self.RightHand`))
    (return (`|MakeArray` (`self.RPunch1`) (`self.RChargedPunch`)))
    (else
      (set `self.HandSceneComponent` (`self.LeftHand`))
      (return (`|MakeArray` _luppercutpunch _luppercutpunch)))))

(fn `Set to Attacking`
  (params (OwnerController :type "/Game/Ai/AIC_EnemyBase Object Reference"))
  (`/Game/Ai/AIC_EnemyBase.SetAlertnessAlerted` OwnerController)
  (`/Game/Ai/AIC_EnemyBase.SetStateInvestigating` OwnerController (`self.K2_GetActorLocation`)))

(fn `SetMaxHealth`
  (params (NewMaxHealth :type "Float (double-precision)"))
  (`/Game/Ai/DamageSystem/BPC_DamageSystem.SetMaxHealth` (`self.BPC_DamageSystem`) NewMaxHealth)
  (return))

(fn `SetMovementSpeed`
  (params (Speed :type "/Game/Ai/BaseEnemy/EnemyBaseEnums/E_AiMovementSpeed Enum" :default "NewEnumerator1"))
  (returns (SpeedValue :type "Float (double-precision)"))
  (bind _output_get (set `CharacterMovementComponent.MaxWalkSpeed` (select `/Game/Ai/BaseEnemy/EnemyBaseEnums/E_AiMovementSpeed` Speed :`NewEnumerator1` 200.0 :`NewEnumerator3` 250.0 :`NewEnumerator6` 300.0 :`NewEnumerator7` 350.0 :`NewEnumerator4` 500.0 :`NewEnumerator5` 300.0 :`NewEnumerator8` 100.0 :!type "Float (single-precision)") (`self.CharacterMovement`)))
  (return _output_get))

(fn `TakeDamage`
  (params (DamageInfo :type "/Game/Ai/DamageSystem/S_DamageInfo Structure"))
  (returns (bWasDamaged :type Boolean))
  (bind (_amountofdamage _damagetype _damageresponse _hitlocation _hitnormal _bonedamaged) (break `/Game/Ai/DamageSystem/S_DamageInfo` DamageInfo))
  (bind _bpc_damagesystem (`self.BPC_DamageSystem`))
  (`GameplayStatics.SpawnDecalAttached` "/Game/Ai/BaseEnemy/BloodVFX/M_Blood_Decal_Inst.M_Blood_Decal_Inst" (`self.BloodDecalSize`) (`self.Mesh`) _bonedamaged _hitlocation (struct) "KeepWorldPosition")
  (`self.BodyPartHit` _hitnormal _bonedamaged
    (:`Head`
      (bind _state (`/Game/Ai/AIC_EnemyBase.GetCurrentState` (cast `/Game/Ai/AIC_EnemyBase` (`self.GetController`) :!pure true)))
      (if (and (`|EnumEquality` _damagetype "NewEnumerator1") (`|EnumInequality` _state "NewEnumerator1"))
        (bind _bwasdamaged (`/Game/Ai/DamageSystem/BPC_DamageSystem.Take Damage` _bpc_damagesystem (make `/Game/Ai/DamageSystem/S_DamageInfo` (`/Game/Ai/DamageSystem/BPC_DamageSystem.MaxHealth` _bpc_damagesystem) _damagetype _damageresponse _hitlocation _hitnormal)))
        (return _bwasdamaged)
        (else
          _)))
    (:`LeftArm`
      (`self.BodyPartHealth` _amountofdamage :!label _label
        (:`Execute`
          _)))
    (:`RightArm`
      (goto _label :!via `Right Arm`))
    (:`LeftLeg`
      (goto _label :!via `Left Leg`))
    (:`RightLeg`
      (goto _label :!via `Right Leg`))
    (:`Stomach`
      _)
    (:`Other`
      _))
  (bind _bwasdamaged_2 (`/Game/Ai/DamageSystem/BPC_DamageSystem.Take Damage` (`self.BPC_DamageSystem`) DamageInfo))
  (return _bwasdamaged_2))

(fn `UserConstructionScript`
  (bind _bpc_damagesystem (`self.BPC_DamageSystem`))
  (add `/Game/Ai/DamageSystem/BPC_DamageSystem.OnDeath` _bpc_damagesystem (`|CreateDelegate` :!event `Death`))
  (add `/Game/Ai/DamageSystem/BPC_DamageSystem.OnDamageResponse` _bpc_damagesystem (`|CreateDelegate` :!event `DamageResponse`))
  (`self.SetMaxHealth` (`self.MaxHealth`)))