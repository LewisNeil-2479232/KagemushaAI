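; Blood drop effect for enemy AI that leaves blood decals where Niagara particles report positions.
; On BeginPlay it passes itself to the Niagara blood system as the particle data callback object.
; Each reported particle spawns a decal at its position, oriented against its velocity and randomly scaled from a tenth to full DecalSize.
; Decals then fade out using configurable delay and duration.
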(event `self.ReceiveBeginPlay`
  (`NiagaraComponent.SetVariableObject` (`self.NS_BloodEffect`) "BP_Blood" self))

(event `self.ReceiveParticleData`
  (params (Data :type "Array of BasicParticleData Structure (by ref)") (NiagaraSystem :type "NiagaraSystem Object Reference") (SimulationPositionOffset :type "Vector Structure (by ref)"))
  (bind _decalsize (`self.DecalSize`))
  (for _array_element Data
    (bind (_position _size _velocity) (break `BasicParticleData` _array_element))
    (bind _returnvalue (`GameplayStatics.SpawnDecalAtLocation` "/Game/Ai/BaseEnemy/BloodVFX/M_Blood_Decal_Inst.M_Blood_Decal_Inst" (`KismetMathLibrary.Conv_DoubleToVector` (`KismetMathLibrary.Lerp` (* _decalsize 0.1) _decalsize (`KismetMathLibrary.RandomFloatInRange` 0.0 1.0))) _position (`KismetMathLibrary.Conv_VectorToRotator` (* _velocity -1.0))))
    (`DecalComponent.SetFadeOut` _returnvalue (`self.FadeOutStartDelay`) (`self.FadeOutDuration`) true)))

(fn `UserConstructionScript`)