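; BPC_DamageSystem is a damage component that tracks health and death state for AI or other actors in the game.
; TakeDamage subtracts incoming damage while alive, flags death and fires OnDeath at zero health, then broadcasts OnDamageResponse with the response type, hit location and normal.
; SetMaxHealth sets a new maximum and refills health to it.
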(fn `SetMaxHealth`
  (params (NewMaxHealth :type "Float (double-precision)"))
  (bind _output_get (set `self.MaxHealth` NewMaxHealth))
  (set `self.Health` _output_get))

(fn `Take Damage`
  (params (DamageInfo :type "/Game/Ai/DamageSystem/S_DamageInfo Structure"))
  (returns (bWasDamaged :type Boolean))
  (bind (_amountofdamage _damagetype _damageresponse _hitlocation _hitnormal) (break `/Game/Ai/DamageSystem/S_DamageInfo` DamageInfo))
  (if (not (`self.bIsDead`))
    (bind _output_get (set `self.Health` (- (`self.Health`) _amountofdamage)))
    (if (<= _output_get 0.0)
      (set `self.bIsDead` true)
      (`self.OnDeath`)
      (`/Engine/EditorBlueprintResources/StandardMacros.DoOnce` false
        (:`Completed`
          _)))
    (`self.OnDamageResponse` _damageresponse _hitlocation _hitnormal)
    (return true)))