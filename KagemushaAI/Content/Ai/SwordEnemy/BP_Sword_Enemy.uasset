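; Sword-wielding enemy that extends a parent enemy with a sheathed sword, melee slashes and a sheath that drops with physics on death.
; BeginPlay attaches the spawned weapon and sheath to thigh sockets, and montage notifies swap the sword between hand and sheath.
; Attacks play a random katana montage whose notifies toggle a looping-timer sphere trace along the blade, damaging one pawn before stopping.
; Unarmed attacks fall back to the parent.
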(event `self.Death`
  (bind _sheathactor (`self.SheathActor`))
  (bind _weaponmesh (`/Game/Ai/Weapons/BP_AIWeapon_Base.WeaponMesh` _sheathactor))
  ;[1 0 1] Death + Drop the sheath
  (`parent.Death`)
  (`self.K2_DetachFromActor` _sheathactor "KeepWorld" "KeepWorld" "KeepWorld")
  (`PrimitiveComponent.SetSimulatePhysics` _weaponmesh true)
  (`PrimitiveComponent.SetCollisionEnabled` _weaponmesh "QueryAndPhysics"))

(event `self.ReceiveBeginPlay`
  ;[1 0 1] Spawn the sword and sheath on the enemy
  (`parent.ReceiveBeginPlay`)
  (bind _returnvalue (`|SpawnActorFromClass` "/Game/Ai/Weapons/BP_Sword_Sheath.BP_Sword_Sheath_C" (`KismetMathLibrary.MakeTransform` (0.0 0.0 0.0)) "Undefined" "MultiplyWithRoot" null null))
  (bind _output_get (set `self.SheathActor` _returnvalue))
  (`self.K2_AttachToComponent` _output_get (`self.Mesh`) "thigh_l_Sheath_Socket" "KeepRelative" "KeepRelative" "KeepRelative" true)
  (bind _returnvalue_2 (`|SpawnActorFromClass` "/Game/Ai/Weapons/BP_Weapon_Sword.BP_Weapon_Sword_C" (`KismetMathLibrary.MakeTransform` (0.0 0.0 0.0)) "Undefined" "MultiplyWithRoot" null null))
  (bind _output_get_2 (set `self.WeaponActor` _returnvalue_2))
  (`self.K2_AttachToComponent` _output_get_2 (`self.Mesh`) "thigh_l_Sword_Sheathed_Socket" "SnapToTarget" "SnapToTarget" "SnapToTarget" true))

(event `/Game/Ai/BPI_EnemyAi.EquipWeapon`
  ;[1 0 1] Enemy wields their sword
  (bind _notifyname (`|PlayMontage` (`self.Mesh`) "/Game/AnimRetarget/RT_UnSheathing_Sword.RT_UnSheathing_Sword")
    (:`OnCompleted`
      (`self.OnWeaponEquipped` :!label _label))
    (:`OnInterrupted`
      (goto _label))
    (:`OnNotifyBegin`
      (switch `name` _notifyname
        (:`WieldSword`
          (`self.K2_AttachToComponent` (`self.WeaponActor`) (`self.Mesh`) "hand_r_Sword_Socket" "SnapToTarget" "SnapToTarget" "SnapToTarget" true)
          (set `self.bIsWieldingWeapon` true)
          (set `self.bUseControllerRotationYaw` true))))))

(event `/Game/Ai/BPI_EnemyAi.UnequipWeapon`
  ;[1 0 1] Enemy sheaths their sword
  (bind _notifyname (`|PlayMontage` (`self.Mesh`) "/Game/AnimRetarget/RT_Sheathing_Sword_Montage.RT_Sheathing_Sword_Montage")
    (:`OnCompleted`
      (`self.OnWeaponUnequipped`))
    (:`OnNotifyBegin`
      (switch `name` _notifyname
        (:`RemoveSword`
          (`self.K2_AttachToComponent` (`self.WeaponActor`) (`self.Mesh`) "thigh_l_Sword_Sheathed_Socket" "SnapToTarget" "SnapToTarget" "SnapToTarget" true)
          (set `self.bIsWieldingWeapon` false)
          (set `self.bUseControllerRotationYaw` false))))))

(event `self.Drop Weapon`
  ;[1 0 1] Adjusting Strafe Radius
  (`parent.Drop Weapon`)
  (`AnimInstance.Montage_Stop` (`SkeletalMeshComponent.GetAnimInstance` (`self.Mesh`)) 0.0 (`self.SelectedAttack`)))

(event `self.Pick Up Weapon`
  ;[1 0 1] Adjusting Strafe Radius
  (`parent.Pick Up Weapon`)
  (set `self.Attack Radius` 150.0)
  (set `self.Defend Radius` 300.0))

(event `/Game/Ai/BPI_EnemyAi.Attack`
  ;[1 0 1] Attack + Hit Trace
  (if (`self.bIsWieldingWeapon`)
    (set `self.bUseControllerRotationYaw` false)
    ;;[1 0 0] Random Attack Selector
    (bind _selectedattack (`self.RandomAttack` (`|MakeArray` (`self.KatanaLowSlash`) (`self.KatanaNormalSlash`) (`self.KatanaHighSpinSlash`) (`self.KatanaSlideSlash`))))
    (bind _notifyname (`|PlayMontage` (`self.Mesh`) _selectedattack)
      (:`OnCompleted`
        (`KismetSystemLibrary.K2_ClearAndInvalidateTimerHandle` (`self.SwordTraceTimerHandle`))
        (set `self.bUseControllerRotationYaw` true :!label _label_2)
        (`self.OnAttackEnd`))
      (:`OnInterrupted`
        (`KismetSystemLibrary.K2_ClearAndInvalidateTimerHandle` (`self.SwordTraceTimerHandle`))
        (`|PlayMontage` (`self.Mesh`) "/Game/Ai/BaseEnemy/EnemyBaseAnimations/DropWeapon.DropWeapon"
          (:`OnCompleted`
            (goto _label_2))))
      (:`OnNotifyBegin`
        (switch `name` _notifyname
          (:`Slash`
            (`self.Start Sword Trace`))
          (:`StopTrace`
            (`KismetSystemLibrary.K2_ClearAndInvalidateTimerHandle` (`self.SwordTraceTimerHandle`))))))
    (else
      (`parent.Attack`))))

(event `Start Sword Trace`
  ;[1 0 1] Attack + Hit Trace
  (bind _returnvalue (`KismetSystemLibrary.K2_SetTimerDelegate` (delegate `Sword Trace Loop`) 0.01 true))
  (set `self.SwordTraceTimerHandle` _returnvalue))

(event `Sword Trace Loop`
  ;[1 0 1] Attack + Hit Trace
  (bind _asbp_weapon_sword (cast `/Game/Ai/Weapons/BP_Weapon_Sword` (`self.WeaponActor`)))
  (bind _outhits (`KismetSystemLibrary.SphereTraceMultiForObjects` :`Start` (`SceneComponent.K2_GetComponentLocation` (`/Game/Ai/Weapons/BP_Weapon_Sword.SwordTopPoint` _asbp_weapon_sword)) :`End` (`SceneComponent.K2_GetComponentLocation` (`/Game/Ai/Weapons/BP_Weapon_Sword.SwordBottomPoint` _asbp_weapon_sword)) :`Radius` 12.0 :`ObjectTypes` (`|MakeArray` "ObjectTypeQuery3" :!type "EObjectTypeQuery Enum") :`DrawDebugType` "ForDuration" :`DrawTime` 1.0))
  (for _array_element _outhits
    (cast `SkeletalMeshComponent` (`.HitComponent` (`GameplayStatics.BreakHitResult` _array_element)))
    (bind (_bblockinghit _binitialoverlap _time _distance _location _impactpoint _normal _impactnormal _physmat _hitactor _hitcomponent _hitbonename) (`GameplayStatics.BreakHitResult` _array_element))
    (message `/Game/Ai/DamageSystem/BPI_Damageable.TakeDamage` _hitactor (make `/Game/Ai/DamageSystem/S_DamageInfo` (`self.SwordDamage`) "NewEnumerator2" "NewEnumerator1" _impactpoint _impactnormal _hitbonename))
    (`KismetSystemLibrary.K2_ClearAndInvalidateTimerHandle` (`self.SwordTraceTimerHandle`))
    (break)))

(fn `UserConstructionScript`
  (`parent.UserConstructionScript`))