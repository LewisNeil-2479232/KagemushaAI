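; BP_PatrolRoute is a level-placed patrol path for AI enemies, drawn with a spline whose points serve as waypoints.
; It tracks the current PatrolIndex and returns that point's world location projected onto the navmesh, with a tall, narrow query extent.
; IncrementPatrolRoute advances the index and resets it to zero on reaching the last spline point, so that final point is never a target.
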(event `IncrementPatrolRoute`
  ;[0 1 1] To create the path, place into the world and then do ALT + drag on the middle point to create the next point, side points are used to change the curvature of the line. MAKE SURE THE HEIGHT IS THE SAME AS THE ENEMIES
  (bind _output_get (set `self.PatrolIndex` (+ (`self.PatrolIndex`) 1)))
  (if (== _output_get (- (`SplineComponent.GetNumberOfSplinePoints` (`self.PatrolRoute`)) 1))
    (set `self.PatrolIndex` 0)))

(fn `GetSplinePointAsWorldPosition`
  (returns (Location :type "Vector Structure"))
  (return (`NavigationSystemV1.K2_ProjectPointToNavigation` (`SplineComponent.GetLocationAtSplinePoint` (`self.PatrolRoute`) (`self.PatrolIndex`) "World") null null (10.0 10.0 250.0))))

(fn `UserConstructionScript`)