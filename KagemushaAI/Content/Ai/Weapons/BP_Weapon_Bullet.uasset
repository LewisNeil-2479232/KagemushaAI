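; Bullet projectile for AI weapons that damages skeletal mesh targets on impact.
; On BeginPlay it passes itself to its Niagara trail as an object variable.
; Hits on the rifle are ignored; skeletal mesh hits send a damage struct with location, inverted normal and bone, while others print the component name.
; After either hit it hides only the mesh, not its children, then destroys itself after a short delay.
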(event `self.ReceiveBeginPlay`
  (`NiagaraComponent.SetVariableObject` (`self.NS_BulletTrail`) "BP_BulletTrail" self))

(event `self.WeaponMesh.OnComponentHit`
  (params (HitComponent :type "PrimitiveComponent Object Reference") (OtherActor :type "Actor Object Reference") (OtherComp :type "PrimitiveComponent Object Reference") (NormalImpulse :type "Vector Structure") (Hit :type "HitResult Structure (by ref)"))
  (bind (_bblockinghit _binitialoverlap _time _distance _location _impactpoint _normal _impactnormal _physmat _hitactor _hitcomponent _hitbonename) (`GameplayStatics.BreakHitResult` Hit))
  (cast `/Game/Ai/Weapons/BP_Weapon_Rifle` _hitactor
    (:`CastFailed`
      (cast `SkeletalMeshComponent` _hitcomponent
        (:`then`
          (message `/Game/Ai/DamageSystem/BPI_Damageable.TakeDamage` _hitactor (make `/Game/Ai/DamageSystem/S_DamageInfo` (`self.BulletDamage`) "NewEnumerator1" "NewEnumerator0" _impactpoint (* _impactnormal -1.0) _hitbonename)))
        (:`CastFailed`
          (`KismetSystemLibrary.PrintString` (`KismetSystemLibrary.GetDisplayName` _hitcomponent))))
      (`SceneComponent.SetVisibility` (`self.WeaponMesh`) false false)
      (`KismetSystemLibrary.Delay` 3.0)
      (`self.K2_DestroyActor`))))

(fn `UserConstructionScript`
  (`parent.UserConstructionScript`))