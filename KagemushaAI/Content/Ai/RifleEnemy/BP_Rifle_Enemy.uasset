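; Rifle-wielding enemy AI character that spawns a rifle onto its hand socket and fires physical bullets, using the parent attack when unarmed.
; Montage notifies drive attacks: Aiming pauses animation, then locks the target's position and stops yaw tracking briefly before Firing.
; Bullets get an impulse along the line through that locked position, extended by shot distance.
; Dropping the weapon interrupts aiming, while pickup resets attack and defend radii.
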(event Custom|Aiming
  ;[1 0 1] Shooting the bullet
  (Variables|/Script/Engine.SkeletalMeshComponent|SetbPauseAnims (Variables|Character|GetMesh) true)
  (Utilities|FlowControl|Delay (Variables|AttackVariables|GetAimingTime))
  (bind _asaic_enemy_base (Utilities|Casting|CastToAIC_EnemyBase (AI|GetAIController self)))
  (bind _attack_target (Variables|/Game/Ai/AIC_EnemyBase.AIC_EnemyBase_C|GetAttack%20Target _asaic_enemy_base)
    (:then
      (Variables|AttackVariables|SetShootLocation (Transformation|GetActorLocation _attack_target))
      (Variables|Default|SetbUseControllerRotationYaw false)
      (Utilities|FlowControl|Delay (Variables|AttackVariables|GetLockedOnTime))
      (Variables|/Script/Engine.SkeletalMeshComponent|SetbPauseAnims (Variables|Character|GetMesh) false))
    (:else
      (Default|CallOnAttackEnd))))

(event EventAttack
  (bind _weaponactor (Variables|Default|GetWeaponActor))
  (bind _returnvalue (Transformation|GetActorLocation _weaponactor))
  ;[1 0 1] Shooting the bullet
  (if (Variables|Default|GetbIsWieldingWeapon)
    (Variables|Default|SetbUseControllerRotationYaw true)
    (bind _notifyname (Animation|Montage|PlayMontage (Variables|Character|GetMesh) (Variables|AnimMontages|GetAiming%20Montage))
      (:OnCompleted
        (Default|CallOnAttackEnd :!label _label))
      (:OnInterrupted
        (Variables|/Script/Engine.SkeletalMeshComponent|SetbPauseAnims (Variables|Character|GetMesh) false)
        (Animation|Montage|PlayMontage (Variables|Character|GetMesh) "/Game/AnimRetarget/RT_DropWeapon.RT_DropWeapon"
          (:OnCompleted
            (Variables|Default|SetbUseControllerRotationYaw true)
            (goto _label))))
      (:OnNotifyBegin
        (switch name _notifyname
          (:Firing
            (bind _shotendlocation (CallFunction|GetShotEndLocation (Transformation|GetActorLocation (Variables|Default|GetWeaponActor)) (Variables|AttackVariables|GetShootLocation)))
            (bind _returnvalue_2 (Game|SpawnActorfromClass "/Game/Ai/Weapons/BP_Weapon_Bullet.BP_Weapon_Bullet_C" (Math|Transform|MakeTransform _returnvalue) "AlwaysSpawn" "MultiplyWithRoot" 0 0))
            (Physics|AddImpulse (Variables|/Game/Ai/Weapons/BP_AIWeapon_Base.BP_AIWeapon_Base_C|GetWeaponMesh _returnvalue_2) (/ (* (- _returnvalue _shotendlocation) -1.0) (Variables|AttackVariables|GetBulletSpeedDivider)) "None" true))
          (:Aiming
            (CallFunction|Aiming)))))
    (else
      (|CallParentFunction))))

(event EventDeath
  ;[1 0 1] Death
  (|CallParentFunction))

(event EventDropWeapon
  (|CallParentFunction)
  (Animation|Montage|MontageStop (Components|SkeletalMesh|GetAnimInstance (Variables|Character|GetMesh)) 0.0 (Variables|AnimMontages|GetAiming%20Montage)))

(event EventEquipWeapon
  (bind _returnvalue (Game|SpawnActorfromClass "/Game/Ai/Weapons/BP_Weapon_Rifle.BP_Weapon_Rifle_C" (Math|Transform|MakeTransform "0, 0, 0") "Undefined" "MultiplyWithRoot" 0 0))
  (bind _output_get (Variables|Default|SetWeaponActor _returnvalue))
  (Transformation|AttachComponentToComponent _output_get (Variables|Character|GetMesh) (Variables|Default|GetWeapon%20Socket%20Name) "KeepRelative" "KeepRelative" "KeepRelative" true)
  (Variables|Default|SetbIsWieldingWeapon true)
  (Default|CallOnWeaponEquipped))

(event EventBeginPlay
  (|CallParentFunction)
  (CallFunction|EquipWeapon))

(event EventPickUpWeapon
  ;[1 0 1] Pick Up Weapon
  (|CallParentFunction)
  (Variables|Default|SetAttack%20Radius 3e+02)
  (Variables|Default|SetDefend%20Radius 6e+02))

(fn ConstructionScript
  (|CallParentFunction))

(fn GetIdealRange
  (return (Variables|Default|GetAttack%20Radius) (Variables|Default|GetDefend%20Radius)))

(fn GetShotEndLocation
  (params (StartLocation :type Vector) (PlayerLocation :type Vector))
  (bind (_x _y _z) (Math|Vector|BreakVector StartLocation))
  (bind (_x_2 _y_2 _z_2) (Math|Vector|BreakVector PlayerLocation))
  (bind _shotdistance (Variables|AttackVariables|GetShotDistance))
  (bind _returnvalue (|(sqrt(((square((x1-x2)))+(square((y1-y2)))))) _x _x_2 _y _y_2))
  (bind _returnvalue_2 (/ _shotdistance _returnvalue))
  (return (Math|Vector|MakeVector (|(((x1-x2)*multiplier)+x2) _x_2 _x _returnvalue_2) (|(((y1-y2)*multiplier)+y2) _returnvalue_2 _y_2 _y) (|(((z1-z2)*multiplier)+z2) _returnvalue_2 _z_2 _z))))